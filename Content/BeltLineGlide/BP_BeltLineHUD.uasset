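; BP_BeltLineHUD is a HUD Blueprint for the BeltLine Glide bike game, meant to show a title, controls and ride stats.
; DrawHUD only casts the owning pawn to BP_BeltLineBike.
; The panel and text drawing nodes, which read the bike's speed, distance, clean passes and penalties, are not connected to execution, so nothing is drawn.
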(event `self.ReceiveDrawHUD`
  (params (SizeX :type Integer) (SizeY :type Integer))
  (bind _asbp_belt_line_bike (cast `/Game/BeltLineGlide/BP_BeltLineBike` (`self.GetOwningPawn`))))

(fn `UserConstructionScript`)