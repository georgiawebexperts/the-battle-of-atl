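; BP_Pedestrian is a pedestrian actor for BeltLineGlide that paces back and forth along world X around its start position.
; BeginPlay stores the start location as PatrolStart.
; Tick moves it frame-rate independently by PatrolSpeed without sweeping, flipping MovingForward whenever X is at or beyond PatrolDistance on either side.
; The overlap event and construction script are empty.
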(event `self.ReceiveBeginPlay`
  (set `self.PatrolStart` (`self.K2_GetActorLocation` self)))

(event `self.ReceiveActorBeginOverlap`
  (params (OtherActor :type "Actor Object Reference")))

(event `self.ReceiveTick`
  (params (DeltaSeconds :type "Float (single-precision)"))
  (bind _patroldistance (`self.PatrolDistance`))
  (bind _x (.x (`self.PatrolStart`)))
  (bind _returnvalue (* (`self.PatrolSpeed`) DeltaSeconds))
  (bind _x_2 (.x (`self.K2_GetActorLocation` self)))
  (`self.K2_AddActorWorldOffset` self (`KismetMathLibrary.MakeVector` (`KismetMathLibrary.SelectFloat` _returnvalue (- 0.0 _returnvalue) (`self.bMovingForward`))) false false)
  (if (or (>= _x_2 (+ _x _patroldistance)) (<= _x_2 (- _x _patroldistance)))
    (set `self.bMovingForward` (not (`self.bMovingForward`)))))

(fn `UserConstructionScript`)