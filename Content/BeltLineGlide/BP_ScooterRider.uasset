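; Scooter rider actor, shown as a cylinder, that glides along its forward vector with a side-to-side weave.
; The construction script adds the scaled cylinder mesh with query and physics collision; an unreachable copy of that setup remains in the event graph.
; Tick offsets the actor without sweep by PatrolSpeed, plus a lateral sine of its world X scaled by CrossingOffset.
; BeginPlay stores the start transform, which nothing here reads.
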(event `self.ReceiveBeginPlay`
  (set `self.StartLocation` (`self.K2_GetActorLocation` self))
  (set `self.StartRotation` (`self.K2_GetActorRotation` self)))

(event `self.ReceiveActorBeginOverlap`
  (params (OtherActor :type "Actor Object Reference")))

(event `self.ReceiveTick`
  (params (DeltaSeconds :type "Float (single-precision)"))
  (`self.K2_AddActorWorldOffset` self (+ (* (`self.GetActorForwardVector` self) (* (`self.PatrolSpeed`) DeltaSeconds)) (* (`self.GetActorRightVector` self) (* (* (`KismetMathLibrary.Sin` (.x (`self.K2_GetActorLocation` self))) (`self.CrossingOffset`)) DeltaSeconds))) false false))

(fn `UserConstructionScript`
  (bind _returnvalue (`self.AddComponentByClass` self "/Script/Engine.StaticMeshComponent" false (`KismetMathLibrary.MakeTransform` (0.0 0.0 0.0))))
  (bind _asstatic_mesh_component (cast `StaticMeshComponent` _returnvalue))
  (`StaticMeshComponent.SetStaticMesh` _asstatic_mesh_component "/Engine/BasicShapes/Cylinder.Cylinder")
  (`SceneComponent.SetWorldScale3D` _asstatic_mesh_component (0.35 0.35 1.2))
  (`PrimitiveComponent.SetCollisionEnabled` _asstatic_mesh_component "QueryAndPhysics"))