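; Player bike character for BeltLineGlide, driven by Enhanced Input for movement, braking by lowering walk speed, and manual reset.
; BeginPlay stores the start transform and adds the input mapping context.
; Overlapping a pedestrian or scooter rider adds a penalty and teleports the bike back to the start, with a short cooldown against repeat hits.
; Tick records speed, counts moving frames as distance score, and runs down the cooldown.
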(event `self.ReceiveBeginPlay`
  (bind _returnvalue (`GameplayStatics.GetPlayerController` self))
  (bind _returnvalue_2 (pcsubsystem `EnhancedInputLocalPlayerSubsystem` _returnvalue))
  (set `self.StartLocation` (`self.K2_GetActorLocation` self))
  (set `self.StartRotation` (`self.K2_GetActorRotation` self))
  (set `self.bBrakeHeld` false)
  (set `self.ResetCooldown` 0.0)
  (`/Engine/EditorBlueprintResources/StandardMacros.IsValid` _returnvalue
    (:`Is Valid`
      (`/Engine/EditorBlueprintResources/StandardMacros.IsValid` _returnvalue_2
        (:`Is Valid`
          (`EnhancedInputSubsystemInterface.AddMappingContext` _returnvalue_2 "/Game/BeltLineGlide/IMC_BeltLine_Default.IMC_BeltLine_Default" 0 (struct)))))))

(event `EnhancedInput|/Game/BeltLineGlide/IA_Move`
  (params (ActionValue :type "Vector2D Structure") (ElapsedSeconds :type "Float (double-precision)") (TriggeredSeconds :type "Float (double-precision)") (InputAction :type "InputAction Object Reference" :default "/Game/BeltLineGlide/IA_Move.IA_Move"))
  (bind (_x _y) (`KismetMathLibrary.BreakVector2D` ActionValue))
  (:`Triggered`
    (set `self.MoveInput` ActionValue)
    (`self.AddMovementInput` (`self.GetActorForwardVector`) _y)
    (`self.AddMovementInput` (`self.GetActorRightVector`) _x)))

(event `self.ReceiveActorBeginOverlap`
  (params (OtherActor :type "Actor Object Reference"))
  (if (<= (`self.ResetCooldown`) 0.0)
    (cast `/Game/BeltLineGlide/BP_Pedestrian` OtherActor
      (:`then`
        _)
      (:`CastFailed`
        (cast `/Game/BeltLineGlide/BP_ScooterRider` OtherActor)))
    (set `self.PenaltyCount` (+ (`self.PenaltyCount`) 1))
    (set `self.ResetCooldown` 1.0)
    (`KismetSystemLibrary.PrintString` self "Penalty: obstacle contact. Returning to the start." true true (struct :`G` 0.66 :`B` 1.0 :`A` 1.0) 3.0)
    (`self.K2_SetActorLocation` self (`self.StartLocation`) false true)
    (`self.K2_SetActorRotation` self (`self.StartRotation`) true)
    (`MovementComponent.StopMovementImmediately` (`self.CharMoveComp`))))

(event `self.ReceiveTick`
  (params (DeltaSeconds :type "Float (single-precision)"))
  (bind _resetcooldown (`self.ResetCooldown`))
  (bind _returnvalue (`KismetMathLibrary.VSize` (`self.GetVelocity` self)))
  (`|ExecutionSequence`
    (:`then_0`
      (set `self.CurrentSpeed` _returnvalue)
      (if (> _returnvalue 0.0)
        (set `self.DistanceScore` (+ (`self.DistanceScore`) 1))))
    (:`then_1`
      (if (> _resetcooldown 0.0)
        (set `self.ResetCooldown` (- _resetcooldown DeltaSeconds))))))

(event `EnhancedInput|/Game/BeltLineGlide/IA_Brake`
  (params (ActionValue :type Boolean) (ElapsedSeconds :type "Float (double-precision)") (TriggeredSeconds :type "Float (double-precision)") (InputAction :type "InputAction Object Reference" :default "/Game/BeltLineGlide/IA_Brake.IA_Brake"))
  (:`Started`
    (set `self.bBrakeHeld` true)
    (set `CharacterMovementComponent.MaxWalkSpeed` 150.0 (`self.CharMoveComp`)))
  (:`Completed`
    (set `self.bBrakeHeld` false)
    (set `CharacterMovementComponent.MaxWalkSpeed` 650.0 (`self.CharMoveComp`))))

(event `EnhancedInput|/Game/BeltLineGlide/IA_Reset`
  (params (ActionValue :type Boolean) (ElapsedSeconds :type "Float (double-precision)") (TriggeredSeconds :type "Float (double-precision)") (InputAction :type "InputAction Object Reference" :default "/Game/BeltLineGlide/IA_Reset.IA_Reset"))
  (:`Started`
    (`self.K2_SetActorLocation` (`self.StartLocation`) false true)
    (`self.K2_SetActorRotation` (`self.StartRotation`) true)
    (`MovementComponent.StopMovementImmediately` (`self.CharMoveComp`))))

(fn `UserConstructionScript`)